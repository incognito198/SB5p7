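; Brick field for an Arkanoid-style game, built in the construction script as an X-by-Y grid of static mesh components.
; A ball hit spawns a burst effect pushed along the reflected ball direction, then swaps the block to the damaged material, which doubles as its hit state.
; A hit on a damaged block destroys it, adds a point and may spawn BP_Bonus.
; Tick prints ball count and destruction progress or completion.
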(event `self.ReceiveHit`
  (params (MyComp :type "PrimitiveComponent Object Reference") (Other :type "Actor Object Reference") (OtherComp :type "PrimitiveComponent Object Reference") (bSelfMoved :type Boolean) (HitLocation :type "Vector Structure") (HitNormal :type "Vector Structure") (NormalImpulse :type "Vector Structure") (Hit :type "HitResult Structure (by ref)"))
  (bind (_relativelocation_x _relativelocation_y) (`KismetMathLibrary.BreakVector` (`SceneComponent.RelativeLocation` MyComp)))
  (bind (_relativelocation_x_2 _relativelocation_y_2) (`KismetMathLibrary.BreakVector` (`SceneComponent.RelativeLocation` MyComp)))
  (set `self.Hit Location` HitLocation)
  (bind _asbp_arcanoid_8_4 (cast `/Game/Task_9_3/BP_Arcanoid_8_4` Other))
  (bind _returnvalue (`NiagaraFunctionLibrary.SpawnSystemAtLocation` "/Game/Task_9_3/NFX_Burst.NFX_Burst" HitLocation))
  (`FXSystemComponent.SetColorParameter` _returnvalue "Color" (struct :`R` 0.385973 :`G` 30.0 :`A` 1.0))
  (`FXSystemComponent.SetVectorParameter` _returnvalue "Wind" (* (`KismetMathLibrary.GetReflectionVector` (`/Game/Task_9_3/BP_Arcanoid_8_4.Directions` _asbp_arcanoid_8_4) HitNormal) 0.02))
  (if (== (`PrimitiveComponent.GetMaterial` MyComp 0) "/Game/Task_9_3/M_Block_Damaged.M_Block_Damaged")
    (`KismetSystemLibrary.PrintString` (`KismetStringLibrary.Concat_StrStr` "Разрушился блок номер" " " (`KismetStringLibrary.Conv_IntToString` (`KismetMathLibrary.Conv_Int64ToInt` (`KismetMathLibrary.Round64` (+ (* 10 (/ _relativelocation_x_2 (`KismetMathLibrary.Conv_IntToDouble` (`self.Padding X`)))) (/ _relativelocation_y_2 (`KismetMathLibrary.Conv_IntToDouble` (`self.Padding Y`))) 1.0))))) true true (struct :`G` 0.002151 :`B` 1.0 :`A` 1.0))
    (`/Engine/EditorBlueprintResources/StandardMacros.IncrementInt` (`self.Points`)
      (:`  `
        (`ActorComponent.K2_DestroyComponent` MyComp)
        (if (`KismetMathLibrary.RandomBoolWithWeight` 0.15)
          (`|SpawnActorFromClass` "/Game/Task_9_3/BP_Bonus.BP_Bonus_C" (`KismetMathLibrary.MakeTransform` (`self.Hit Location`)) "AlwaysSpawn" "OverrideRootScale" null null))))
    (else
      (`PrimitiveComponent.SetMaterial` MyComp 0 "/Game/Task_9_3/M_Block_Damaged.M_Block_Damaged")
      (`KismetSystemLibrary.PrintString` (`KismetStringLibrary.Concat_StrStr` "Цвет сменился у блока номер" " " (`KismetStringLibrary.Conv_IntToString` (`KismetMathLibrary.Conv_Int64ToInt` (`KismetMathLibrary.Round64` (+ (* 10 (/ _relativelocation_x (`KismetMathLibrary.Conv_IntToDouble` (`self.Padding X`)))) (/ _relativelocation_y (`KismetMathLibrary.Conv_IntToDouble` (`self.Padding Y`))) 1.0))))) true true (struct :`R` 1.0 :`G` 0.029832 :`A` 1.0)))))

(event `self.ReceiveTick`
  (params (DeltaSeconds :type "Float (single-precision)"))
  (bind _outactors (`GameplayStatics.GetAllActorsOfClass` "/Game/Task_9_3/BP_Arcanoid_8_4.BP_Arcanoid_8_4_C"))
  (`KismetSystemLibrary.PrintString` (`KismetStringLibrary.Concat_StrStr` "Количество шариков " " " (`KismetStringLibrary.Conv_IntToString` (`KismetArrayLibrary.Array_Length` _outactors))) true true (struct :`R` 0.946939 :`G` 1.0 :`A` 1.0) DeltaSeconds)
  (if (== (`self.Points`) (* (`self.X`) (`self.Y`)))
    (`KismetSystemLibrary.PrintString` "Вы уничтожили все блоки!" true true (struct :`R` 0.041679 :`G` 1.0 :`B` 0.016521 :`A` 1.0) DeltaSeconds)
    (else
      (`KismetSystemLibrary.PrintString` (`KismetStringLibrary.Concat_StrStr` "Вы уничтожили " (`KismetStringLibrary.Conv_IntToString` (`self.Points`)) " блоков") true true (struct :`R` 1.0 :`B` 0.021061 :`A` 1.0) DeltaSeconds))))

(fn `UserConstructionScript`
  (for _index (range (+ (`self.X`) 1))
    (for _index_2 (range (+ (`self.Y`) 1))
      (`AddComponent|NODE_AddStaticMeshComponent-0` :`RelativeTransform` (`KismetMathLibrary.MakeTransform` (`KismetMathLibrary.MakeVector` (`KismetMathLibrary.Conv_IntToDouble` (* _index (`self.Padding X`))) (`KismetMathLibrary.Conv_IntToDouble` (* _index_2 (`self.Padding Y`)))) (struct) (1.0 2.0 1.0))))))