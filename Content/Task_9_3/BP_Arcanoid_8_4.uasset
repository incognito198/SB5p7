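; BP_Arcanoid_8_4 is the ball of an Arkanoid-style game, held at the BP_Platform capsule with a "Press Space" prompt until Ready is set.
; Once ready, Tick moves it by swept offsets and reflects its direction off the normal of blocking hits.
; Entering a KillZVolume spawns a Niagara burst and destroys the ball, calling OnDead if no balls remain.
; Destroyed-object counting and speed reduction logic is present but unconnected.
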(event `self.ReceiveBeginPlay`
  (`KismetSystemLibrary.Delay` 0.1)
  (set `self.CurrentSpeed` (`self.BaseSpeed`)))

(event `self.ReceiveTick`
  (params (DeltaSeconds :type "Float (single-precision)"))
  (if (`self.Ready?`)
    (bind _sweephitresult (`self.K2_AddActorWorldOffset` (* (* (`self.Directions`) (`self.CurrentSpeed`)) DeltaSeconds) true))
    (bind (_bblockinghit _binitialoverlap _time _distance _location _impactpoint _normal) (`GameplayStatics.BreakHitResult` _sweephitresult))
    (if _bblockinghit
      (set `self.Directions` (`KismetMathLibrary.GetReflectionVector` (`self.Directions`) (`KismetMathLibrary.MakeVector` (.x _normal) (.y _normal)))))
    (else
      (`KismetSystemLibrary.PrintString` "Press Space. Get ready!" true true (struct :`R` 1.0 :`B` 0.014251 :`A` 1.0) DeltaSeconds)
      (bind _outactors (`GameplayStatics.GetAllActorsOfClass` "/Game/Task_9_3/BP_Platform.BP_Platform_C"))
      (bind _capsule (`/Game/Task_9_3/BP_Platform.Capsule` (`|GetArrayItem` _outactors)))
      (bind (_returnvalue_location _returnvalue_rotation) (`KismetMathLibrary.BreakTransform` (`SceneComponent.K2_GetComponentToWorld` _capsule)))
      (`SceneComponent.K2_SetWorldTransform` (`self.Sphere`) (`KismetMathLibrary.MakeTransform` _returnvalue_location _returnvalue_rotation (`SceneComponent.RelativeScale3D` _capsule)) false false))))

(event `self.ReceiveActorBeginOverlap`
  (params (OtherActor :type "Actor Object Reference"))
  (cast `KillZVolume` OtherActor)
  (bind _returnvalue (`NiagaraFunctionLibrary.SpawnSystemAtLocation` "/Game/Task_9_3/NFX_Burst.NFX_Burst" (`SceneComponent.K2_GetComponentLocation` (`self.Sphere`))))
  (`FXSystemComponent.SetColorParameter` _returnvalue "Color" (struct :`G` 1.114383 :`B` 30.0 :`A` 1.0))
  (set `self.Ready?` false)
  (`self.K2_DestroyActor`)
  (bind _outactors (`GameplayStatics.GetAllActorsOfClass` "BP_Arcanoid_8_4_C"))
  (if (== (`KismetArrayLibrary.Array_Length` _outactors) 0)
    (`self.OnDead`)))

(fn `UserConstructionScript`)