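; BP_Bonus is a moving pickup for an Arkanoid-style game that duplicates the balls in play.
; It moves every tick along its direction at its speed with a swept offset, and destroys itself on overlapping the platform or a kill volume.
; A platform hit first gathers all balls and spawns a ready copy at each one's DubliSpawn transform, unless over 32 exist, when it prints a warning instead.
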(event `self.ReceiveTick`
  (params (DeltaSeconds :type "Float (single-precision)"))
  (`self.K2_AddActorWorldOffset` (* (* (`self.Direction`) (`self.Speed`)) DeltaSeconds) true))

(event `self.Sphere.OnComponentBeginOverlap`
  (params (OverlappedComponent :type "PrimitiveComponent Object Reference") (OtherActor :type "Actor Object Reference") (OtherComp :type "PrimitiveComponent Object Reference") (OtherBodyIndex :type Integer) (bFromSweep :type Boolean) (SweepResult :type "HitResult Structure (by ref)"))
  (cast `/Game/Task_9_3/BP_Platform` OtherActor
    (:`then`
      (bind _outactors (`GameplayStatics.GetAllActorsOfClass` "/Game/Task_9_3/BP_Arcanoid_8_4.BP_Arcanoid_8_4_C"))
      (set `self.PresentBalls` _outactors)
      (`self.SpawnDubli`))
    (:`CastFailed`
      (cast `KillZVolume` OtherActor)))
  (`self.K2_DestroyActor`))

(event `SpawnDubli`
  (bind _returnvalue (`KismetArrayLibrary.Array_Length` (`self.PresentBalls`)))
  (if (<= _returnvalue 32)
    (for _index (range (+ _returnvalue 1))
      (bind (_returnvalue_location _returnvalue_rotation _returnvalue_scale) (`KismetMathLibrary.BreakTransform` (`SceneComponent.K2_GetComponentToWorld` (`/Game/Task_9_3/BP_Arcanoid_8_4.DubliSpawn` (`|GetArrayItem` (`self.PresentBalls`) _index)))))
      (bind _returnvalue_2 (`|SpawnActorFromClass` "/Game/Task_9_3/BP_Arcanoid_8_4.BP_Arcanoid_8_4_C" (`KismetMathLibrary.MakeTransform` _returnvalue_location _returnvalue_rotation _returnvalue_scale) "AdjustIfPossibleButAlwaysSpawn" "OverrideRootScale" null null))
      (set `/Game/Task_9_3/BP_Arcanoid_8_4.Ready?` true _returnvalue_2))
    (else
      (`KismetSystemLibrary.PrintString` "Достаточно шариков, а то комп взорвется" true true (struct :`R` 1.0 :`B` 0.015653 :`A` 100.0) 4.0))))

(fn `UserConstructionScript`)