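; Player paddle for an Arkanoid-style game that slides sideways in fixed, swept steps from axis input and launches the ball.
; On BeginPlay, SpawnBall creates a BP_Arcanoid_8_4 ball at the capsule if none exists and binds to its OnDead event.
; Space sets the ball's Ready flag.
; Ball hits on the cube spawn a colored Niagara effect, its wind driven by the ball's direction reflected about the hit normal.
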(event `Key|SpaceBar`
  (params (Key :type "Key Structure"))
  (:`Pressed`
    (bind _outactors (`GameplayStatics.GetAllActorsOfClass` "/Game/Task_9_3/BP_Arcanoid_8_4.BP_Arcanoid_8_4_C"))
    (set `/Game/Task_9_3/BP_Arcanoid_8_4.Ready?` true (`|GetArrayItem` _outactors))))

(event `InputAxis|MoveRightProject`
  (params (AxisValue :type "Float (single-precision)"))
  (if (< AxisValue 0.0)
    (`self.K2_AddActorWorldOffset` (0.0 -50.0 0.0) true)))

(event `InputAxis|MoveRightProject`
  (params (AxisValue :type "Float (single-precision)"))
  (if (> AxisValue 0.0)
    (`self.K2_AddActorWorldOffset` (0.0 50.0 0.0) true)))

(event `self.ReceiveBeginPlay`
  (`self.SpawnBall`))

(event `self.Cube.OnComponentHit`
  (params (HitComponent :type "PrimitiveComponent Object Reference") (OtherActor :type "Actor Object Reference") (OtherComp :type "PrimitiveComponent Object Reference") (NormalImpulse :type "Vector Structure") (Hit :type "HitResult Structure (by ref)"))
  (bind (_bblockinghit _binitialoverlap _time _distance _location _impactpoint _normal) (`GameplayStatics.BreakHitResult` Hit))
  (bind _asbp_arcanoid_8_4 (cast `/Game/Task_9_3/BP_Arcanoid_8_4` OtherActor))
  (bind _returnvalue (`NiagaraFunctionLibrary.SpawnSystemAtLocation` "/Game/Task_9_3/NFX_Platform.NFX_Platform" _location (struct) (2.0 2.0 2.0)))
  (`FXSystemComponent.SetVectorParameter` _returnvalue "Wind" (* (`KismetMathLibrary.GetReflectionVector` (`/Game/Task_9_3/BP_Arcanoid_8_4.Directions` _asbp_arcanoid_8_4) _normal) 0.005))
  (`FXSystemComponent.SetColorParameter` _returnvalue "Color" (struct :`R` 30.0 :`B` 18.204388 :`A` 1.0)))

(fn `SpawnBall`
  (bind _capsule (`self.Capsule`))
  (bind (_returnvalue_location _returnvalue_rotation) (`KismetMathLibrary.BreakTransform` (`SceneComponent.K2_GetComponentToWorld` _capsule)))
  (bind _outactors (`GameplayStatics.GetAllActorsOfClass` "/Game/Task_9_3/BP_Arcanoid_8_4.BP_Arcanoid_8_4_C"))
  (if (== (`KismetArrayLibrary.Array_Length` _outactors) 0)
    (bind _returnvalue (`|SpawnActorFromClass` "/Game/Task_9_3/BP_Arcanoid_8_4.BP_Arcanoid_8_4_C" (`KismetMathLibrary.MakeTransform` _returnvalue_location (`KismetMathLibrary.MakeRotator` (.roll _returnvalue_rotation) (.pitch _returnvalue_rotation) (+ (.yaw _returnvalue_rotation) 90.0)) (`SceneComponent.RelativeScale3D` _capsule)) "AlwaysSpawn" "OverrideRootScale" null null))
    (bind _output_get (set `self.PlayingBall` _returnvalue))
    (add `/Game/Task_9_3/BP_Arcanoid_8_4.OnDead` _output_get (`|CreateDelegate` :!event `SpawnBall`))
    (return)))

(fn `UserConstructionScript`)