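; BP_Arcanoid is a self-moving actor for an Arkanoid-style mechanic that bounces off surfaces and destroys what it hits.
; Each tick it sweeps along its direction at the current speed, reflecting the direction about the hit normal on blocking hits.
; Any valid hit actor is destroyed and counted, and speed drops by a tenth of base speed while the result stays above the minimum.
; The count and speed print on screen every frame.
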(event `self.ReceiveBeginPlay`
  (set `self.CurrentSpeed` (`self.BaseSpeed`)))

(event `self.ReceiveTick`
  (params (DeltaSeconds :type "Float (single-precision)"))
  (bind _currentspeed (`self.CurrentSpeed`))
  (bind _returnvalue (- (`self.CurrentSpeed`) (* (`self.BaseSpeed`) 0.1)))
  (`KismetSystemLibrary.PrintString` (`KismetStringLibrary.Concat_StrStr` (`KismetStringLibrary.Conv_IntToString` (`self.Number of Destroyed Objects`)) "_______" (`KismetStringLibrary.Conv_DoubleToString` _currentspeed)) true true (`self.Text Color`) DeltaSeconds)
  (bind _sweephitresult (`self.K2_AddActorWorldOffset` (* (* (`self.Directions`) _currentspeed) DeltaSeconds) true))
  (bind (_bblockinghit _binitialoverlap _time _distance _location _impactpoint _normal _impactnormal _physmat _hitactor) (`GameplayStatics.BreakHitResult` _sweephitresult))
  (if _bblockinghit
    (set `self.Directions` (`KismetMathLibrary.GetReflectionVector` (`self.Directions`) _normal))
    (`/Engine/EditorBlueprintResources/StandardMacros.IsValid` _hitactor
      (:`Is Valid`
        (`self.K2_DestroyActor` _hitactor)
        (`/Engine/EditorBlueprintResources/StandardMacros.IncrementInt` (`self.Number of Destroyed Objects`)
          (:`  `
            (if (< (`self.MinimalSpeed`) _returnvalue)
              (set `self.CurrentSpeed` _returnvalue))))))))

(fn `UserConstructionScript`)