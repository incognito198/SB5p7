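; BP_SmartLight is a spot light actor that blinks a configurable number of times when play begins.
; BeginPlay applies the configured color, then a looped wire toggles intensity between full and zero with an adjustable delay, counting cycles until the blink limit.
; A disconnected for-loop that delays and prints its index never runs.
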(event `self.ReceiveBeginPlay`
  (bind _spotlight (`self.SpotLight`))
  (`LightComponent.SetLightColor` (`self.SpotLight`) (`self.New Light Color`) true)
  (`LightComponent.SetIntensity` _spotlight 100000.0 :!label _label)
  (`KismetSystemLibrary.Delay` (`self.Delay`))
  (`LightComponent.SetIntensity` _spotlight 0.0)
  (`KismetSystemLibrary.Delay` (`self.Delay`))
  (bind _result (`/Engine/EditorBlueprintResources/StandardMacros.IncrementInt` (`self.LoopCounter`))
    (:`  `
      (if (not (== _result (`self.NumberOfBlinks`)))
        (goto _label)))))

(fn `UserConstructionScript`)