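; BP_Arcanoid_7_3 is an Arkanoid-style moving actor that bounces off whatever blocks it.
; Each Tick it makes a swept move along Directions at CurrentSpeed, reflects the direction on the hit normal, and prints a destroyed-object count and speed.
; The hit-actor validity check leads nowhere; logic to increment the count and lower speed toward a minimum is disconnected and never runs.
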(event `self.ReceiveBeginPlay`
  (set `self.CurrentSpeed` (`self.BaseSpeed`)))

(event `self.ReceiveTick`
  (params (DeltaSeconds :type "Float (single-precision)"))
  (bind _currentspeed (`self.CurrentSpeed`))
  (`KismetSystemLibrary.PrintString` (`KismetStringLibrary.Concat_StrStr` (`KismetStringLibrary.Conv_IntToString` (`self.Number of Destroyed Objects`)) "_______" (`KismetStringLibrary.Conv_DoubleToString` _currentspeed)) true true (`self.Text Color`) DeltaSeconds)
  (bind _sweephitresult (`self.K2_AddActorWorldOffset` (* (* (`self.Directions`) _currentspeed) DeltaSeconds) true))
  (bind (_bblockinghit _binitialoverlap _time _distance _location _impactpoint _normal _impactnormal _physmat _hitactor) (`GameplayStatics.BreakHitResult` _sweephitresult))
  (if _bblockinghit
    (set `self.Directions` (`KismetMathLibrary.GetReflectionVector` (`self.Directions`) _normal))
    (`/Engine/EditorBlueprintResources/StandardMacros.IsValid` _hitactor)))

(fn `UserConstructionScript`)