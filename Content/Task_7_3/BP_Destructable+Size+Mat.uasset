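; BP_Destructable+Size+Mat is a child actor Blueprint that gives its Cube a random material whenever another actor begins overlapping it.
; On overlap it picks an entry from the MaterialMassive array, applies it to element 0, then calls the parent's overlap logic.
; The random range's upper bound is the array length rather than the last index, so it can select an out-of-range entry.
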(event `self.ReceiveActorBeginOverlap`
  (params (OtherActor :type "Actor Object Reference"))
  (bind _materialmassive (`self.MaterialMassive`))
  (`/Engine/EditorBlueprintResources/StandardMacros.IsValid` self
    (:`Is Valid`
      (`PrimitiveComponent.SetMaterial` (`self.Cube`) 0 (`|GetArrayItem` _materialmassive (`KismetMathLibrary.RandomIntegerInRange` 0 (`KismetArrayLibrary.Array_Length` _materialmassive))))
      (`parent.ReceiveActorBeginOverlap` OtherActor))))

(fn `UserConstructionScript`
  (`parent.UserConstructionScript`))