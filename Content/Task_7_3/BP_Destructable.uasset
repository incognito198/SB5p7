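; BP_Destructable is a destructible actor for an Arkanoid task that breaks after a set number of overlaps with BP_Arcanoid_7_3.
; Each overlap on its Cube increments a counter after a short Delay, which also drops overlaps that arrive during the wait.
; When the count equals the required hit number, the actor destroys itself and prints a message, while Tick shows current progress on screen every frame.
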(event `self.ReceiveTick`
  (params (DeltaSeconds :type "Float (single-precision)"))
  (`KismetSystemLibrary.PrintString` (`KismetStringLibrary.Concat_StrStr` "Количество пересечений" " " (`KismetStringLibrary.Conv_IntToString` (`self.ammount of overlaps`)) " " "из" " " (`KismetStringLibrary.Conv_IntToString` (`self.Number of hits to destr`))) true true (struct :`R` 1.0 :`B` 0.992671 :`A` 1.0) DeltaSeconds))

(event `self.Cube.OnComponentBeginOverlap`
  (params (OverlappedComponent :type "PrimitiveComponent Object Reference") (OtherActor :type "Actor Object Reference") (OtherComp :type "PrimitiveComponent Object Reference") (OtherBodyIndex :type Integer) (bFromSweep :type Boolean) (SweepResult :type "HitResult Structure (by ref)"))
  (cast `/Game/Task_7_3/BP_Arcanoid_7_3` OtherActor)
  (`KismetSystemLibrary.Delay` 0.2)
  (bind _result (`/Engine/EditorBlueprintResources/StandardMacros.IncrementInt` (`self.ammount of overlaps`))
    (:`  `
      (if (== _result (`self.Number of hits to destr`))
        (`self.K2_DestroyActor`)
        (`KismetSystemLibrary.PrintString` "Объект уничтожен" true true (struct :`R` 0.057249 :`G` 1.0 :`A` 1.0))))))

(fn `UserConstructionScript`)